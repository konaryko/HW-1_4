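; BP_Actor is a test actor that prints the contents of the DT_Items data table, apparently as a task exercise labelled "Задание 3".
; On BeginPlay it loops over every row name in DT_Items, looks up each row and prints its Name on screen in blue.
; Tick is empty, and a forward visibility line trace with debug drawing is left unconnected, so it never runs.
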(event `self.ReceiveBeginPlay`
  (bind _outrownames (`DataTableFunctionLibrary.GetDataTableRowNames` "/Game/BluePrints/Core/DT_Items.DT_Items"))
  (for _array_element _outrownames
    (bind _returnvalue (`|GetDataTableRow` "/Game/BluePrints/Core/DT_Items.DT_Items" _array_element)
      (:`then`
        (`KismetSystemLibrary.PrintString` (`KismetTextLibrary.Conv_TextToString` (`|FormatText` "Задание 3 - Data Table: {Name}" (`.Name_6_3A48E13041EDAF1BBE77E9AFBCD25416` (break `/Game/BluePrints/Core/S_ItemName` _returnvalue)))) true true (struct :`G` 0.074973 :`B` 1.0 :`A` 1.0) 10.0)))))

(event `self.ReceiveTick`
  (params (DeltaSeconds :type "Float (single-precision)")))

(fn `UserConstructionScript`)