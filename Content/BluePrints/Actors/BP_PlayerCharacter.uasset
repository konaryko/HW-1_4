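; Player character with mouse-aimed facing and three switchable guns, in the style of a top-down shooter.
; Enhanced Input drives movement along the actor's axes and jumping.
; Each tick, control yaw turns at constant speed toward the cursor ray's intersection with a horizontal plane at the character.
; Keys 1–3 select which projectile class spawns at Point when shooting; an older line-trace damage path is disconnected.
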(event `self.ReceiveBeginPlay`
  ; MovementBase
  (bind _asplayer_controller (cast `PlayerController` (`self.GetController`)))
  (`EnhancedInputSubsystemInterface.AddMappingContext` (pcsubsystem `EnhancedInputLocalPlayerSubsystem` _asplayer_controller) "/Game/BluePrints/Input/IMC_FP.IMC_FP" 0 (struct))
  (set `self.Value1 ` 1.0))

(event `EnhancedInput|/Game/BluePrints/Input/IA_Walk`
  (params (ActionValue :type "Vector2D Structure") (ElapsedSeconds :type "Float (double-precision)") (TriggeredSeconds :type "Float (double-precision)") (InputAction :type "InputAction Object Reference" :default "/Game/BluePrints/Input/IA_Walk.IA_Walk"))
  ; MovementControl
  (:`Triggered`
    (`KismetSystemLibrary.PrintString` (`KismetTextLibrary.Conv_TextToString` (`|FormatText` " X: {x}" ActionValue_X)) true true (struct :`G` 0.66 :`B` 1.0 :`A` 1.0) 0.0)
    (`self.AddMovementInput` (`KismetMathLibrary.GetForwardVector` (`self.K2_GetActorRotation`)) ActionValue_X true)
    (`KismetSystemLibrary.PrintString` (`KismetTextLibrary.Conv_TextToString` (`|FormatText` " Y: {y}" ActionValue_Y)) true true (struct :`G` 0.66 :`B` 1.0 :`A` 1.0) -0.0)
    (`self.AddMovementInput` (`KismetMathLibrary.GetRightVector` (`self.K2_GetActorRotation`)) ActionValue_Y)))

(event `EnhancedInput|/Game/BluePrints/Input/IA_Jump`
  (params (ActionValue :type "Vector2D Structure") (ElapsedSeconds :type "Float (double-precision)") (TriggeredSeconds :type "Float (double-precision)") (InputAction :type "InputAction Object Reference" :default "/Game/BluePrints/Input/IA_Jump.IA_Jump"))
  (:`Started`
    (`self.Jump`))
  (:`Completed`
    (`self.StopJumping`)))

(event `self.ReceiveTick`
  (params (DeltaSeconds :type "Float (single-precision)"))
  (bind (_worldlocation _worlddirection) (`PlayerController.DeprojectMousePositionToWorld` (`GameplayStatics.GetPlayerController` 0)))
  (bind (_returnvalue_roll _returnvalue_pitch _returnvalue_yaw) (`KismetMathLibrary.BreakRotator` (`KismetMathLibrary.RInterpTo_Constant` (`self.K2_GetActorRotation`) (`KismetMathLibrary.FindLookAtRotation` (`self.K2_GetActorLocation`) (`.Intersection` (`KismetMathLibrary.LinePlaneIntersection_OriginNormal` _worldlocation (+ _worldlocation (* _worlddirection 5000)) (`self.K2_GetActorLocation`) (0.0 0.0 1.0)))) (`GameplayStatics.GetWorldDeltaSeconds`) 720.0)))
  ; CameraControl
  (`Controller.SetControlRotation` (`self.GetController`) (`KismetMathLibrary.MakeRotator` 0.0 0.0 _returnvalue_yaw)))

(event `EnhancedInput|/Game/BluePrints/Input/IA_Shooting`
  (params (ActionValue :type Boolean) (ElapsedSeconds :type "Float (double-precision)") (TriggeredSeconds :type "Float (double-precision)") (InputAction :type "InputAction Object Reference" :default "/Game/BluePrints/Input/IA_Shooting.IA_Shooting"))
  ; LineTrace
)

(event `EnhancedInput|/Game/BluePrints/Input/IA_Shooting`
  (params (ActionValue :type Boolean) (ElapsedSeconds :type "Float (double-precision)") (TriggeredSeconds :type "Float (double-precision)") (InputAction :type "InputAction Object Reference" :default "/Game/BluePrints/Input/IA_Shooting.IA_Shooting"))
  (bind (_returnvalue_location _returnvalue_rotation) (`KismetMathLibrary.BreakTransform` (`SceneComponent.K2_GetComponentToWorld` (`self.Point `))))
  (bind (_returnvalue_location_2 _returnvalue_rotation_2) (`KismetMathLibrary.BreakTransform` (`SceneComponent.K2_GetComponentToWorld` (`self.Point `))))
  (bind (_returnvalue_location_3 _returnvalue_rotation_3) (`KismetMathLibrary.BreakTransform` (`SceneComponent.K2_GetComponentToWorld` (`self.Point `))))
  (:`Triggered`
    (`KismetSystemLibrary.PrintString` "Shooting!" true true (struct :`R` 1.0 :`A` 1.0) 0.0)
    (bind _output_get (set `self.Boolean` (== 1.0 (`self.Value1 `))))
    (if _output_get
      (`|SpawnActorFromClass` "/Game/BluePrints/Actors/Weapon/BP_BaseProjectile.BP_BaseProjectile_C" (`KismetMathLibrary.MakeTransform` _returnvalue_location_2 _returnvalue_rotation_2) "Undefined" "MultiplyWithRoot" null null)
      (else
        (bind _output_get_2 (set `self.Boolean` (== 2.0 (`self.Value1 `))))
        (if _output_get_2
          (`|SpawnActorFromClass` "/Game/BluePrints/Actors/Weapon/BP_BaseProjectile_Child.BP_BaseProjectile_Child_C" (`KismetMathLibrary.MakeTransform` _returnvalue_location_3 _returnvalue_rotation_3) "Undefined" "MultiplyWithRoot" null null)
          (else
            (`|SpawnActorFromClass` "/Game/BluePrints/Actors/Weapon/BP_BaseProjectile_Child2.BP_BaseProjectile_Child2_C" (`KismetMathLibrary.MakeTransform` _returnvalue_location _returnvalue_rotation) "Undefined" "MultiplyWithRoot" null null)))))))

(event `Key|One`
  (params (Key :type "Key Structure"))
  (:`Pressed`
    (`KismetSystemLibrary.PrintString` "Gun 1!" true true (struct :`R` 1.0 :`A` 1.0) 3.0)
    (set `self.Value1 ` 1.0)))

(event `Key|Two`
  (params (Key :type "Key Structure"))
  (:`Pressed`
    (`KismetSystemLibrary.PrintString` "Gun 2!" true true (struct :`R` 1.0 :`A` 1.0) 3.0)
    (set `self.Value1 ` 2.0)))

(event `Key|Three`
  (params (Key :type "Key Structure"))
  (:`Pressed`
    (`KismetSystemLibrary.PrintString` "Gun 3!" true true (struct :`R` 1.0 :`A` 1.0) 3.0)
    (set `self.Value1 ` 3.0)))

(fn `UserConstructionScript`)