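; BP_Trigger is a box trigger actor that appears to be a learning exercise, printing Russian-labelled numbered task results.
; Player overlap turns on its point light and increments a crossing counter; any end overlap turns it off, without a player check.
; Each counted entry also prints the DT_Items "Granate" row via DTShow.
; Calculator then prints the doubled count, decremented and truncated, labelled as a sum.
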(event `self.Box.OnComponentBeginOverlap`
  (params (OverlappedComponent :type "PrimitiveComponent Object Reference") (OtherActor :type "Actor Object Reference") (OtherComp :type "PrimitiveComponent Object Reference") (OtherBodyIndex :type Integer) (bFromSweep :type Boolean) (SweepResult :type "HitResult Structure (by ref)"))
  (cast `/Game/BluePrints/Actors/BP_PlayerCharacter` OtherActor)
  (set `self.InRadius?` true)
  (if (`self.InRadius?`) :!label _label
    (`LightComponent.SetIntensity` (`self.PointLight`) 1000.0)
    (bind _output_get (set `self.InRadiusCount` (+ (`self.InRadiusCount`) 1)))
    (`KismetSystemLibrary.PrintString` (`KismetTextLibrary.Conv_TextToString` (`|FormatText` "Задание 1 - Количество пересечений: {In Radius Count} " _output_get)) true true (struct :`R` 1.0 :`B` 0.671823 :`A` 1.0) 10.0)
    (`self.DT_Show`)
    (`self.Calculator`)
    (else
      (`LightComponent.SetIntensity` (`self.PointLight`) 0.0))))

(event `self.Box.OnComponentEndOverlap`
  (params (OverlappedComponent :type "PrimitiveComponent Object Reference") (OtherActor :type "Actor Object Reference") (OtherComp :type "PrimitiveComponent Object Reference") (OtherBodyIndex :type Integer))
  (set `self.InRadius?` false)
  (goto _label))

(fn `Calculator`
  (bind _result (`/Engine/EditorBlueprintResources/StandardMacros.DecrementFloat` (`KismetMathLibrary.Conv_IntToDouble` (+ (`self.InRadiusCount`) (`self.InRadiusCount`))))
    (:`  `
      (bind _output_get (set `self.Result ` (`KismetMathLibrary.FTrunc` _result)))
      (`KismetSystemLibrary.PrintString` (`KismetTextLibrary.Conv_TextToString` (`|FormatText` "Задание 5 - Результат сложения: {Result}" _output_get))))))

(fn `DT_Show`
  (`DataTableFunctionLibrary.GetDataTableRowNames` "/Game/BluePrints/Core/DT_Items.DT_Items")
  (bind _returnvalue (`|GetDataTableRow` "/Game/BluePrints/Core/DT_Items.DT_Items" "Granate")
    (:`then`
      (bind (_name _count _yes_no) (break `/Game/BluePrints/Core/S_ItemName` _returnvalue))
      (`KismetSystemLibrary.PrintText` (`|FormatText` "Задание 4 - {1} | {0} | {2} " _name _count _yes_no)))))

(fn `UserConstructionScript`)